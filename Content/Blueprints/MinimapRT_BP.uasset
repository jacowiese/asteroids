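; MinimapRT_BP is a minimap helper that follows the player's ship and feeds the minimap image in the main UI.
; Every tick it casts to the player ship controller and its controlled ship, then moves its Scene component to the ship mesh's world location without changing rotation.
; In the same tick it reassigns the render target material as the minimap image's brush, rather than setting it once.
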(event `self.ReceiveTick`
  (params (DeltaSeconds :type "Float (single-precision)"))
  (bind _asplayer_ship_controller_bp (cast `/Game/Blueprints/PlayerShipController_BP` (`GameplayStatics.GetPlayerController` 0)))
  (bind _asplayer_ship_bp (cast `/Game/Blueprints/PlayerShip_BP` (`Controller.K2_GetPawn` _asplayer_ship_controller_bp)))
  (`SceneComponent.K2_SetWorldLocation` (`self.Scene`) (`SceneComponent.K2_GetComponentLocation` (`/Game/Blueprints/PlayerShip_BP.Mesh` _asplayer_ship_bp)) false false)
  (`Image.SetBrushFromMaterial` (`/Game/UI/PlayerUI.MinimapImage` (`/Game/Blueprints/PlayerShipController_BP.MainUIWidget` _asplayer_ship_controller_bp)) "/Game/Minimap/MinimapRenderTarget_Mat.MinimapRenderTarget_Mat"))

(fn `UserConstructionScript`)