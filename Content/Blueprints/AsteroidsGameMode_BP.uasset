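; Game mode for an Asteroids-style level that spawns and tracks asteroids in a square playfield, drawn as a debug box.
; On BeginPlay it scatters extra-large asteroids at random points, and Tick declares the level complete once the tracked array empties, currently just printing a message.
; A separate helper spawns an asteroid of a given type near a location with random planar velocity and adds it to the array.
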(event `self.ReceiveBeginPlay`
  ;[1 1 1] Spawn Initial Asteroids
  (`self.SpawnLevelAsteroids` (`self.NumberOfAsteroids`))
  (set `self.GameInPlay` true))

(event `self.ReceiveTick`
  (params (DeltaSeconds :type "Float (single-precision)"))
  (bind _playfieldsize (`self.PlayfieldSize`))
  ;[1 1 1] GameMode Event Tick
  (`KismetSystemLibrary.DrawDebugBox` (0.0 0.0 0.0) (`KismetMathLibrary.MakeVector` _playfieldsize _playfieldsize 250.0) (struct :`R` 0.04964 :`G` 1.0 :`A` 1.0))
  (if (`self.GameInPlay`)
    (if (<= (`KismetArrayLibrary.Array_Length` (`self.Asteroids`)) 0)
      (set `self.GameInPlay` false)
      (`self.LevelComplete`))))

(event `LevelComplete`
  (`KismetSystemLibrary.PrintString` "All asteroids destroyed, level complete!"))

(fn `SpawnAsteroidAtLocation`
  (params (SpawnLocation :type "Vector Structure") (AsteroidType :type "EAsteroidType Enum"))
  (returns (Asteroid :type "/Game/Blueprints/Asteroid_BP Object Reference"))
  (bind (_returnvalue_x _returnvalue_y) (`KismetMathLibrary.BreakVector` (`KismetMathLibrary.RandomUnitVector`)))
  (bind (_returnvalue_x_2 _returnvalue_y_2) (`KismetMathLibrary.BreakVector` (+ SpawnLocation (`KismetMathLibrary.RandomUnitVector`))))
  (bind _returnvalue (`|SpawnActorFromClass` "/Game/Blueprints/Asteroid_BP.Asteroid_BP_C" (`KismetMathLibrary.MakeTransform` (`KismetMathLibrary.MakeVector` _returnvalue_x_2 _returnvalue_y_2)) "AdjustIfPossibleButAlwaysSpawn" "OverrideRootScale"))
  (`Asteroid.InitialiseAsteroid` _returnvalue AsteroidType)
  (`PrimitiveComponent.SetPhysicsLinearVelocity` (`StaticMeshActor.StaticMeshComponent` _returnvalue) (* (`KismetMathLibrary.MakeVector` (- _returnvalue_x 0.5) (- _returnvalue_y 0.5)) (`KismetMathLibrary.RandomFloatInRange` 5.0 15.0)) false "None")
  (`KismetArrayLibrary.Array_Add` (`self.Asteroids`) _returnvalue)
  (return _returnvalue))

(fn `SpawnLevelAsteroids`
  (params (NumberOfAsteroidsToSpawn :type Integer))
  (bind (_returnvalue_x _returnvalue_y) (`KismetMathLibrary.BreakVector` (* (`KismetMathLibrary.RandomUnitVector`) (`self.PlayfieldSize`))))
  (for _ (range 1 (+ NumberOfAsteroidsToSpawn 1))
    (bind _returnvalue (`|SpawnActorFromClass` "/Game/Blueprints/Asteroid_BP.Asteroid_BP_C" (`KismetMathLibrary.MakeTransform` (`KismetMathLibrary.MakeVector` _returnvalue_x _returnvalue_y)) "AdjustIfPossibleButAlwaysSpawn" "OverrideRootScale"))
    (`Asteroid.InitialiseAsteroid` _returnvalue "XLARGE")
    (`KismetArrayLibrary.Array_Add` (`self.Asteroids`) _returnvalue))
  (return))

(fn `UserConstructionScript`)