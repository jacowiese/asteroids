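; Player controller for a ship game that creates the player UI and routes input to the player ship pawn.
; Turn and camera axes rotate the ship and its camera gimbal, while fire and thrust presses set held flags.
; Tick uses those flags to thrust, toggle thruster effects and fire the main weapon.
; It also scales the spring arm length with ship speed, clamped, so the camera pulls back when moving fast.
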(event `self.ReceiveBeginPlay`
  (bind _returnvalue (`|CreateWidget` "/Game/UI/PlayerUI.PlayerUI_C"))
  (`UserWidget.AddToViewport` _returnvalue 0)
  (set `self.MainUIWidget` _returnvalue))

(event `InputAction|Fire`
  (params (Key :type "Key Structure" :default "AnyKey"))
  ;[1 1 1] Weapon Input
  (:`Pressed`
    (set `self.FirePressed` true))
  (:`Released`
    (set `self.FirePressed` false)))

(event `InputAxis|Turn`
  (params (AxisValue :type "Float (single-precision)"))
  ;[1 1 1] Ship Turning Input
  (bind _returnvalue (`self.GetPlayerShip`))
  (`PlayerShip.RotateShip` _returnvalue AxisValue))

(event `InputAction|Thrust`
  (params (Key :type "Key Structure" :default "AnyKey"))
  ;[1 1 1] Ship Thrusting Input
  (:`Pressed`
    (set `self.ThrustPressed` true))
  (:`Released`
    (set `self.ThrustPressed` false)))

(event `self.ReceiveTick`
  (params (DeltaSeconds :type "Float (single-precision)"))
  (bind _playershipbp (`self.GetPlayerShipBP`))
  ;[1 1 1] Event Tick
  (`|ExecutionSequence`
    (:`then_0`
      (if (`self.ThrustPressed`)
        (bind _returnvalue (`self.GetPlayerShip`))
        (`PlayerShip.ThrustShip` _returnvalue 1.0)
        (`/Game/Blueprints/PlayerShip_BP.ActivateThrusters` (`self.GetPlayerShipBP`) true)
        (else
          (`/Game/Blueprints/PlayerShip_BP.ActivateThrusters` (`self.GetPlayerShipBP`) false))))
    (:`then_1`
      (set `SpringArmComponent.TargetArmLength` (`KismetMathLibrary.FClamp` (* (`KismetMathLibrary.VSize` (`self.GetVelocity` _playershipbp)) 2.0) 800.0 2500.0) (`/Game/Blueprints/PlayerShip_BP.SpringArm` _playershipbp)))
    (:`then_2`
      (if (`self.FirePressed`)
        (`PlayerShip.FireMainWeapon` (`self.GetPlayerShipBP`))))))

(event `InputAxis|RotateCamera`
  (params (AxisValue :type "Float (single-precision)"))
  ;[1 1 1] Camera Rotation
  (`SceneComponent.K2_AddLocalRotation` (`/Game/Blueprints/PlayerShip_BP.Gymbal` (`self.GetPlayerShipBP`)) (`KismetMathLibrary.MakeRotator` 0.0 0.0 (* (`KismetMathLibrary.FClamp` AxisValue -1.0 1.0) (* (`GameplayStatics.GetWorldDeltaSeconds`) (`self.CameraRotationRate`)))) false false))

(fn `GetPlayerShipBP`
  (returns (PlayerShipBP :type "/Game/Blueprints/PlayerShip_BP Object Reference"))
  (bind _asplayer_ship_bp (cast `/Game/Blueprints/PlayerShip_BP` (`GameplayStatics.GetPlayerPawn` 0)))
  (return _asplayer_ship_bp))

(fn `UserConstructionScript`)