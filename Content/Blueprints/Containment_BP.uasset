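; Containment actor that builds a circular field of GasCloudBlocker_BP actors around the world origin on BeginPlay.
; It always spawns a dense outer ring at one-degree steps, then scatters progressively smaller inner rings using a random modulo test, dropping spawns that still collide after adjustment.
; GetCircleLocation adds slight XY jitter at zero height, and its combined sine/cosine terms make rings √2 times the given radius.
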(event `self.ReceiveBeginPlay`
  (`|ExecutionSequence`
    (:`then_0`
      (for _index (range 360)
        (bind _returnvalue (`|SpawnActorFromClass` "/Game/Blueprints/GasCloudBlocker_BP.GasCloudBlocker_BP_C" (`KismetMathLibrary.MakeTransform` (`self.GetCircleLocation` (`KismetMathLibrary.Conv_IntToDouble` _index) (`self.Radius`)) (`KismetMathLibrary.RandomRotator` true)) "AlwaysSpawn" "OverrideRootScale" null null))
        (`KismetArrayLibrary.Array_Add` (`self.Blockers`) _returnvalue)))
    (:`then_1`
      (for _index_2 (range 1 81)
        (for _index_3 (range 360)
          (if (== (mod _index_3 (`KismetMathLibrary.RandomIntegerInRange` 2 20)) 0)
            (bind _returnvalue_2 (`|SpawnActorFromClass` "/Game/Blueprints/GasCloudBlocker_BP.GasCloudBlocker_BP_C" (`KismetMathLibrary.MakeTransform` (`self.GetCircleLocation` (`KismetMathLibrary.Conv_IntToDouble` _index_3) (- (`self.Radius`) (* (`KismetMathLibrary.Conv_IntToDouble` _index_2) 10.0))) (`KismetMathLibrary.RandomRotator` true)) "AdjustIfPossibleButDontSpawnIfColliding" "OverrideRootScale" null null))
            (`KismetArrayLibrary.Array_Add` (`self.Blockers`) _returnvalue_2)))))))

(fn `GetCircleLocation`
  (params (Degree :type "Float (double-precision)") (Radius :type "Float (double-precision)"))
  (returns (Location :type "Vector Structure"))
  (bind (_returnvalue_x _returnvalue_y) (`KismetMathLibrary.BreakVector` (* (`KismetMathLibrary.RandomUnitVector`) 5.0)))
  (return (+ (`KismetMathLibrary.MakeVector` (+ (* (`KismetMathLibrary.DegSin` Degree) Radius) (* Radius (`KismetMathLibrary.DegCos` Degree))) (- (* Radius (`KismetMathLibrary.DegCos` Degree)) (* (`KismetMathLibrary.DegSin` Degree) Radius))) (`KismetMathLibrary.MakeVector` _returnvalue_x _returnvalue_y))))

(fn `UserConstructionScript`)