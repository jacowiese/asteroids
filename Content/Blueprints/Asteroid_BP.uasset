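; Asteroid actor for an Asteroids-style game that drifts with a random planar velocity, tumbles, and wraps around the playfield edges.
; Projectile hits pass their damage to TakeHit, then destroy the projectile.
; When destroyed, non-small asteroids have the game mode spawn two of the next smaller type at their location.
; Every destroyed asteroid removes itself from the game mode's Asteroids list.
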(event `self.ReceiveBeginPlay`
  (bind (_returnvalue_x _returnvalue_y) (`KismetMathLibrary.BreakVector` (`KismetMathLibrary.RandomUnitVector`)))
  (set `self.Rotation` (`KismetMathLibrary.RandomUnitVector`))
  (`PrimitiveComponent.SetPhysicsLinearVelocity` (`self.StaticMeshComponent`) (* (`KismetMathLibrary.MakeVector` (- _returnvalue_x 0.5) (- _returnvalue_y 0.5)) (`KismetMathLibrary.RandomFloatInRange` 1.0 15.0)) false "None"))

(event `self.ReceiveTick`
  (params (DeltaSeconds :type "Float (single-precision)"))
  (bind _playfieldsize (`self.GetPlayfieldSize`))
  (bind _playfieldsize_2 (`self.GetPlayfieldSize`))
  (bind (_returnvalue_x _returnvalue_y _returnvalue_z) (`KismetMathLibrary.BreakVector` (`SceneComponent.K2_GetComponentLocation` (`self.StaticMeshComponent`))))
  (bind (_returnvalue_x_2 _returnvalue_y_2 _returnvalue_z_2) (`KismetMathLibrary.BreakVector` (`SceneComponent.K2_GetComponentLocation` (`self.StaticMeshComponent`))))
  (`SceneComponent.K2_AddRelativeRotation` (`self.StaticMeshComponent`) (`KismetMathLibrary.MakeRotator` (.x (* (`self.Rotation`) (* (`self.RotationScale`) DeltaSeconds))) (.y (* (`self.Rotation`) (* (`self.RotationScale`) DeltaSeconds))) (.z (* (`self.Rotation`) (* (`self.RotationScale`) DeltaSeconds)))) false false)
  (if (< _returnvalue_x_2 (- 0.0 _playfieldsize_2))
    (`self.K2_SetActorLocation` (`KismetMathLibrary.MakeVector` (`self.GetPlayfieldSize`) _returnvalue_y_2 _returnvalue_z_2))
    (elif (> _returnvalue_x_2 _playfieldsize_2)
      (`self.K2_SetActorLocation` (`KismetMathLibrary.MakeVector` (- 0.0 (`self.GetPlayfieldSize`)) _returnvalue_y_2 _returnvalue_z_2))
      (elif (< _returnvalue_y (- 0.0 _playfieldsize))
        (`self.K2_SetActorLocation` (`KismetMathLibrary.MakeVector` _returnvalue_x (`self.GetPlayfieldSize`) _returnvalue_z))
        (elif (> _returnvalue_y _playfieldsize)
          (`self.K2_SetActorLocation` (`KismetMathLibrary.MakeVector` _returnvalue_x (- 0.0 (`self.GetPlayfieldSize`)) _returnvalue_z)))))))

(event `self.ReceiveHit`
  (params (MyComp :type "PrimitiveComponent Object Reference") (Other :type "Actor Object Reference") (OtherComp :type "PrimitiveComponent Object Reference") (bSelfMoved :type Boolean) (HitLocation :type "Vector Structure") (HitNormal :type "Vector Structure") (NormalImpulse :type "Vector Structure") (Hit :type "HitResult Structure (by ref)"))
  (bind _asprojectile_bp (cast `/Game/Blueprints/Projectile_BP` Other))
  (`|ExecutionSequence`
    (:`then_0`
      (bind _returnvalue (`Projectile.GetProjectileDamage` _asprojectile_bp))
      (`self.TakeHit` _returnvalue)
      (`KismetSystemLibrary.PrintString` (`KismetStringLibrary.BuildString_Double` "" "Asteroid took " _returnvalue " damage.")))
    (:`then_1`
      (`self.K2_DestroyActor` _asprojectile_bp))))

(event `self.OnAsteroidDestroyed`
  (bind _returnvalue (`self.K2_GetActorLocation`))
  (bind _tempasteroidtype (`self.TempAsteroidType`))
  (switch `EAsteroidType` (`self.asteroidType`)
    (:`SMALL`
      (bind _asasteroids_game_mode_bp (cast `/Game/Blueprints/AsteroidsGameMode_BP` (`GameplayStatics.GetGameMode`) :!label _label))
      (`KismetArrayLibrary.Array_RemoveItem` (`/Game/Blueprints/AsteroidsGameMode_BP.Asteroids` _asasteroids_game_mode_bp) self)
      (`self.K2_DestroyActor`))
    (:`MEDIUM`
      (set `self.TempAsteroidType` "SMALL")
      (`|ExecutionSequence` :!label _label_2
        (:`then_0`
          (bind _asasteroids_game_mode_bp_2 (cast `/Game/Blueprints/AsteroidsGameMode_BP` (`GameplayStatics.GetGameMode`)))
          (`/Game/Blueprints/AsteroidsGameMode_BP.SpawnAsteroid` _asasteroids_game_mode_bp_2 _returnvalue _tempasteroidtype))
        (:`then_1`
          (`/Game/Blueprints/AsteroidsGameMode_BP.SpawnAsteroid` _asasteroids_game_mode_bp_2 _returnvalue _tempasteroidtype))
        (:`then_2`
          (goto _label))))
    (:`LARGE`
      (set `self.TempAsteroidType` "MEDIUM")
      (goto _label_2))
    (:`XLARGE`
      (set `self.TempAsteroidType` "LARGE")
      (goto _label_2))))

(fn `GetPlayfieldSize`
  (returns (PlayfieldSize :type "Float (double-precision)"))
  (bind _asasteroids_game_mode_bp (cast `/Game/Blueprints/AsteroidsGameMode_BP` (`GameplayStatics.GetGameMode`)))
  (return (`/Game/Blueprints/AsteroidsGameMode_BP.PlayfieldSize` _asasteroids_game_mode_bp)))

(fn `UserConstructionScript`)