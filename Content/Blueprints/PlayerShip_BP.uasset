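; Player ship for an Asteroids-style game that stays inside a square, wrap-around playfield.
; Each tick, WrapToPlayfield reads PlayfieldSize from AsteroidsGameMode_BP and teleports the ship to the opposite edge when its mesh crosses an X or Y bound, one axis per tick.
; Hitting an asteroid plays a bump sound at that asteroid's location.
; ActivateThrusters switches the left and right thruster components on or off together.
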(event `self.ReceiveTick`
  (params (DeltaSeconds :type "Float (single-precision)"))
  (`self.WrapToPlayfield`))

(event `self.ReceiveHit`
  (params (MyComp :type "PrimitiveComponent Object Reference") (Other :type "Actor Object Reference") (OtherComp :type "PrimitiveComponent Object Reference") (bSelfMoved :type Boolean) (HitLocation :type "Vector Structure") (HitNormal :type "Vector Structure") (NormalImpulse :type "Vector Structure") (Hit :type "HitResult Structure (by ref)"))
  ;[1 1 1] Ship Collisions
  ;;[1 1 1] Asteroid
  (bind _asasteroid_bp (cast `/Game/Blueprints/Asteroid_BP` Other))
  (`GameplayStatics.PlaySoundAtLocation` "/Game/Sounds/ship_rock_bump.ship_rock_bump" (`self.K2_GetActorLocation` _asasteroid_bp)))

(fn `ActivateThrusters`
  (params (ActiveState :type Boolean))
  (`ActorComponent.SetActive` (`self.Right Thruster`) ActiveState false)
  (`ActorComponent.SetActive` (`self.Left Thruster`) ActiveState false)
  (return))

(fn `GetPlayfieldSize`
  (returns (PlayfieldSize :type "Float (double-precision)"))
  (bind _asasteroids_game_mode_bp (cast `/Game/Blueprints/AsteroidsGameMode_BP` (`GameplayStatics.GetGameMode`))
    (:`then`
      _)
    (:`CastFailed`
      (`KismetSystemLibrary.PrintText` "Cast error : Get Playfield Size")))
  (return (`/Game/Blueprints/AsteroidsGameMode_BP.PlayfieldSize` _asasteroids_game_mode_bp)))

(fn `UserConstructionScript`)

(fn `WrapToPlayfield`
  (bind _playfieldsize (`self.GetPlayfieldSize`))
  (bind _playfieldsize_2 (`self.GetPlayfieldSize`))
  (bind (_returnvalue_x _returnvalue_y _returnvalue_z) (`KismetMathLibrary.BreakVector` (`SceneComponent.K2_GetComponentLocation` (`self.Mesh`))))
  (bind (_returnvalue_x_2 _returnvalue_y_2 _returnvalue_z_2) (`KismetMathLibrary.BreakVector` (`SceneComponent.K2_GetComponentLocation` (`self.Mesh`))))
  (if (< _returnvalue_x (- 0.0 _playfieldsize))
    (`self.K2_SetActorLocation` (`KismetMathLibrary.MakeVector` (`self.GetPlayfieldSize`) _returnvalue_y _returnvalue_z))
    (elif (> _returnvalue_x _playfieldsize)
      (`self.K2_SetActorLocation` (`KismetMathLibrary.MakeVector` (- 0.0 (`self.GetPlayfieldSize`)) _returnvalue_y _returnvalue_z))
      (elif (< _returnvalue_y_2 (- 0.0 _playfieldsize_2))
        (`self.K2_SetActorLocation` (`KismetMathLibrary.MakeVector` _returnvalue_x_2 (`self.GetPlayfieldSize`) _returnvalue_z_2))
        (elif (> _returnvalue_y_2 _playfieldsize_2)
          (`self.K2_SetActorLocation` (`KismetMathLibrary.MakeVector` _returnvalue_x_2 (- 0.0 (`self.GetPlayfieldSize`)) _returnvalue_z_2))))))
  (return))